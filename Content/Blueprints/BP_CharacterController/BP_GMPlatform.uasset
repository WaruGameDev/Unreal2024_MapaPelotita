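; BP_GMPlatform, a game mode by its name, sets up the HUD and holds health and money values.
; BeginPlay creates the score and life bar widgets, adds both to the viewport and stores the life bar as HealthBar.
; Tick pushes HP and HpMax to the bar through CalculateBar every frame.
; GainMoney adds an amount to Money without notifying either widget.
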(event `self.ReceiveBeginPlay`
  (bind _returnvalue (`|CreateWidget` "/Game/Blueprints/UI/WBP_Score.WBP_Score_C"))
  (`UserWidget.AddToViewport` _returnvalue 0)
  (bind _returnvalue_2 (`|CreateWidget` "/Game/Blueprints/UI/WBP_LifeBAR.WBP_LifeBAR_C"))
  (`UserWidget.AddToViewport` _returnvalue_2 0)
  (set `self.HealthBar` _returnvalue_2))

(event `self.ReceiveTick`
  (params (DeltaSeconds :type "Float (single-precision)"))
  (`/Game/Blueprints/UI/WBP_LifeBAR.CalculateBar` (`self.HealthBar`) (`self.HP`) (`self.HpMax`)))

(event `/Game/Blueprints/Inteface/BPI_GainMoney.GainMoney`
  (params (amount :type Integer))
  (set `self.Money` (+ (`self.Money`) amount)))

(fn `UserConstructionScript`)