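; BP_Turret is an interactable turret that fires bullets continuously from the moment play begins.
; A Shoot timeline, with its play rate set from FireRate, slides the Canon component along X to animate each shot.
; When the timeline finishes, it spawns a BP_Bullet at the cannon facing the actor's rotation, plays an explosion effect and sound, then restarts itself as the firing loop.
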(event `self.ReceiveBeginPlay`
  (bind _returnvalue (`SceneComponent.K2_GetComponentLocation` (`self.canon`)))
  (`TimelineComponent.SetPlayRate` (`self.Shoot`) (`self.FireRate`))
  (bind (_direction _shootpos) (`Timeline|Shoot` :!via `PlayFromStart` :!label _label)
    (:`Update`
      (`SceneComponent.K2_SetRelativeLocation` (`self.canon`) (`KismetMathLibrary.MakeVector` (+ _shootpos 80.0)) false false))
    (:`Finished`
      (`|SpawnActorFromClass` "/Game/Blueprints/Interactables/BP_Bullet.BP_Bullet_C" (`KismetMathLibrary.MakeTransform` _returnvalue (`self.K2_GetActorRotation` self)) "Undefined" "MultiplyWithRoot" null null)
      (`GameplayStatics.SpawnEmitterAtLocation` "/Game/StarterContent/Particles/P_Explosion.P_Explosion" _returnvalue)
      (`GameplayStatics.PlaySoundAtLocation` "/Game/StarterContent/Audio/Explosion01.Explosion01" _returnvalue (struct) 1.0 1.0 0.0 null null null null)
      (goto _label :!via `PlayFromStart`))))

(fn `UserConstructionScript`)