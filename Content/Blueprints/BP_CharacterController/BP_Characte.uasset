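; Paper2D player character for the grandma figure, with Enhanced Input movement, jumping and flipbook animation.
; BeginPlay adds the puzzle-game mapping context; despite its name, IA_Rotate drives world-space X/Y movement, with Y inverted.
; Every tick, X velocity flips and tilts the sprite to face travel.
; Tick also selects walk or idle flipbooks from planar velocity, then overrides them with rise or fall flipbooks while airborne.
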(event `self.ReceiveBeginPlay`
  (bind _asbp_character_controller_pc (cast `/Game/Blueprints/BP_CharacterController/BP_CharacterControllerPC` (`GameplayStatics.GetPlayerController` 0)))
  (`EnhancedInputSubsystemInterface.AddMappingContext` (pcsubsystem `EnhancedInputLocalPlayerSubsystem` _asbp_character_controller_pc) "/Game/Input/IMC_Puzzleame.IMC_Puzzleame" 0 (struct)))

(event `EnhancedInput|/Game/Input/IA_Rotate`
  (params (ActionValue :type "Vector2D Structure") (ElapsedSeconds :type "Float (double-precision)") (TriggeredSeconds :type "Float (double-precision)") (InputAction :type "InputAction Object Reference" :default "/Game/Input/IA_Rotate.IA_Rotate"))
  (:`Triggered`
    (`self.AddMovementInput` (`KismetMathLibrary.MakeVector` ActionValue_X (* ActionValue_Y -1.0)))))

(event `EnhancedInput|/Game/Input/IA_Jump`
  (params (ActionValue :type Boolean) (ElapsedSeconds :type "Float (double-precision)") (TriggeredSeconds :type "Float (double-precision)") (InputAction :type "InputAction Object Reference" :default "/Game/Input/IA_Jump.IA_Jump"))
  (:`Triggered`
    (`self.Jump`))
  (:`Canceled`
    (`self.StopJumping`)))

(event `self.ReceiveTick`
  (params (DeltaSeconds :type "Float (single-precision)"))
  (`self.Set Player Rotation`)
  (`self.SetRunAndIdleAnimation`)
  (`self.JumpAnimation`))

(event `Set Player Rotation`
  (bind _sprite (`self.Sprite`))
  (bind _velocity_x (`KismetMathLibrary.BreakVector` (`MovementComponent.Velocity` (`self.CharacterMovement`))))
  (if (< _velocity_x 0.0)
    (`SceneComponent.K2_SetRelativeRotation` _sprite (struct :`Roll` -35.0) false false)
    (elif (> _velocity_x 0.0)
      (`SceneComponent.K2_SetRelativeRotation` _sprite (struct :`Yaw` 180.0 :`Roll` 35.0) false false))))

(event `SetRunAndIdleAnimation`
  (bind _sprite (`self.Sprite`))
  (bind (_velocity_x _velocity_y) (`KismetMathLibrary.BreakVector` (`MovementComponent.Velocity` (`self.CharacterMovement`))))
  (if (> (+ (`KismetMathLibrary.Abs` _velocity_x) (`KismetMathLibrary.Abs` _velocity_y)) 0.0)
    (`PaperFlipbookComponent.SetFlipbook` _sprite "/Game/2D/PF_WalkGrandMa.PF_WalkGrandMa")
    (else
      (`PaperFlipbookComponent.SetFlipbook` _sprite "/Game/2D/PF_IdleGrandma.PF_IdleGrandma"))))

(event `JumpAnimation`
  (bind _charactermovement (`self.CharacterMovement`))
  (bind _sprite (`self.Sprite`))
  (bind (_velocity_x _velocity_y _velocity_z) (`KismetMathLibrary.BreakVector` (`MovementComponent.Velocity` _charactermovement)))
  (if (`NavMovementComponent.IsMovingOnGround` _charactermovement)
    _
    (elif (> _velocity_z 0.0)
      (`PaperFlipbookComponent.SetFlipbook` _sprite "/Game/2D/FB_upGrandma_Flipbook.FB_upGrandma_Flipbook")
      (else
        (`PaperFlipbookComponent.SetFlipbook` _sprite "/Game/2D/FB_DownGrandma_Flipbook.FB_DownGrandma_Flipbook")))))

(fn `UserConstructionScript`)