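; BP_Bullet is a projectile that damages the player on contact and destroys itself five seconds after spawning.
; Each tick it moves along its local X axis by Speed, without delta-time scaling, so travel rate depends on frame rate.
; When Sphere1 begins overlapping the player pawn, it decrements HP on the BP_GMPlatform game mode, and the bullet keeps flying after the hit.
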(event `self.ReceiveTick`
  (params (DeltaSeconds :type "Float (single-precision)"))
  (`self.K2_AddActorLocalOffset` (`KismetMathLibrary.MakeVector` (`self.Speed`))))

(event `self.ReceiveBeginPlay`
  (`KismetSystemLibrary.Delay` 5.0)
  (`self.K2_DestroyActor`))

(event `self.Sphere1.OnComponentBeginOverlap`
  (params (OverlappedComponent :type "PrimitiveComponent Object Reference") (OtherActor :type "Actor Object Reference") (OtherComp :type "PrimitiveComponent Object Reference") (OtherBodyIndex :type Integer) (bFromSweep :type Boolean) (SweepResult :type "HitResult Structure (by ref)"))
  (if (== OtherActor (`GameplayStatics.GetPlayerPawn` 0))
    (bind _asbp_gmplatform (cast `/Game/Blueprints/BP_CharacterController/BP_GMPlatform` (`GameplayStatics.GetGameMode`)))
    (`/Engine/EditorBlueprintResources/StandardMacros.DecrementFloat` (`/Game/Blueprints/BP_CharacterController/BP_GMPlatform.HP` _asbp_gmplatform))))

(fn `UserConstructionScript`)